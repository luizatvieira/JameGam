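; Enemy character that patrols destination points, chases the player on sight and calls the player's kill event on reaching them.
; PawnSensing sightings trigger an AI MoveTo chase and switch the peripheral vision angle.
; Each tick, visibility line traces across an arc feed a procedural mesh that draws the field of view, separately from detection.
; A respawn event teleports the enemy to its first destination.
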(event `OnPlayerRespawn`
  ;[1 1 1] On Player Respawn
  (`self.K2_SetActorTransform` (`KismetMathLibrary.Conv_VectorToTransform` (`self.RespawnPosition`)) false true))

(event `self.ReceiveBeginPlay`
  ;[1 1 1] Initialize
  (set `CharacterMovementComponent.MaxWalkSpeed` (`self.Max Walk Speed`) (`self.CharacterMovement`))
  (`self.OnPatrol` self)
  (set `self.RespawnPosition` (`|GetArrayItem` (`self.Destinations`))))

(event `self.ReceiveTick`
  (params (DeltaSeconds :type "Float (single-precision)"))
  (`self.UpdateFOV` self)
  (`self.Draw View Lines` self))

(event `OnPatrol`
  (bind _destinationindex (`self.DestinationIndex`))
  ;[1 1 1] Patrol
  (if (not (`self.IsSeeingPlayer?`))
    (`|AIMoveTo` self (`|GetArrayItem` (`self.Destinations`) (`self.DestinationIndex`)) null
      (:`OnSuccess`
        (`KismetSystemLibrary.Delay` (`KismetMathLibrary.RandomFloatInRange` 4.5 5.0))
        (`/Engine/EditorBlueprintResources/StandardMacros.IncrementInt` _destinationindex
          (:`  `
            (if (== _destinationindex (`self.TotalDestinations`))
              (set `self.DestinationIndex` 0)
              (`self.OnPatrol`))))))
    (else
      (`self.OnPatrol`))))

(event `self.PlayerSensing.OnSeePawn`
  (params (Pawn :type "Pawn Object Reference"))
  ;[1 1 1] Player Follow
  (set `self.IsSeeingPlayer?` true)
  (`self.OnPlayerFollow`))

(event `OnPlayerFollow`
  (bind _returnvalue (`GameplayStatics.GetPlayerCharacter` 0))
  ;[1 1 1] Player Follow
  (if (`self.IsSeeingPlayer?`)
    (`PawnSensingComponent.SetPeripheralVisionAngle` (`self.PlayerSensing`) (`self.ActiveVisionAngle`))
    (`|AIMoveTo` self (0.0 0.0 0.0) _returnvalue
      (:`OnSuccess`
        (bind _asbp_character (cast `/Game/Characters/BP_Character` _returnvalue))
        (`/Game/Characters/BP_Character.OnPlayerKilled` _asbp_character)))
    (else
      (set `self.IsSeeingPlayer?` false)
      (`PawnSensingComponent.SetPeripheralVisionAngle` (`self.PlayerSensing`) (`self.InactiveVisionAngle`))
      (`MovementComponent.StopMovementImmediately` (`self.CharacterMovement`)))))

(fn `CreateProceduralMesh`
  (locals (LLeftPoint :type "Vector Structure") (LRightPoint :type "Vector Structure") (j :type Integer))
  (bind (_bblockinghit _binitialoverlap _time _distance _location _impactpoint _normal _impactnormal _physmat _hitactor _hitcomponent _hitbonename _bonename _hititem _elementindex _faceindex _tracestart _traceend) (`GameplayStatics.BreakHitResult` (`|GetArrayItem` (`self.Out Hit`))))
  (bind (_bblockinghit_2 _binitialoverlap_2 _time_2 _distance_2 _location_2 _impactpoint_2 _normal_2 _impactnormal_2 _physmat_2 _hitactor_2 _hitcomponent_2 _hitbonename_2 _bonename_2 _hititem_2 _elementindex_2 _faceindex_2 _tracestart_2 _traceend_2) (`GameplayStatics.BreakHitResult` (`|GetArrayItem` (`self.Out Hit`) (+ (`local.j`) 1))))
  (for _index (range (`KismetArrayLibrary.Array_LastIndex` (`self.Out Hit`)))
    (set `local.j` _index)
    (`|ExecutionSequence`
      (:`then_0`
        (if _bblockinghit
          (set `local.LLeftPoint` _location)
          (else
            (set `local.LLeftPoint` _traceend))))
      (:`then_1`
        (if _bblockinghit_2
          (set `local.LRightPoint` _location_2)
          (else
            (set `local.LRightPoint` _traceend_2))))
      (:`then_2`
        (`ProceduralMeshComponent.CreateMeshSection_LinearColor` :`self` (`self.ProceduralMesh`) :`Vertices` (`|MakeArray` (- (`self.StartDrawPoint`) (`self.StartDrawPoint`)) (- (`local.LLeftPoint`) (`self.StartDrawPoint`)) (- (`local.LRightPoint`) (`self.StartDrawPoint`))) :`Triangles` (`|MakeArray` 0 2 1))
        (`PrimitiveComponent.SetMaterial` (`self.ProceduralMesh`) (`local.j`) "/Game/StarterContent/Particles/Materials/m_flare_01.m_flare_01"))))
  (`SceneComponent.K2_SetRelativeRotation` (`self.ProceduralMesh`) (* (`KismetMathLibrary.MakeRotFromX` (`self.GetActorForwardVector`)) -1.0) false false))

(fn `Draw View Lines`
  (bind _startdrawpoint (`self.StartDrawPoint`))
  (for _index (range (+ (`self.NumberOfSections`) 1))
    (set `self.LCurrentAngle` (- (* _index (`self.DAngle`)) (`self.HalfAngle`)))
    (bind _outhit (`KismetSystemLibrary.LineTraceSingle` :`Start` _startdrawpoint :`End` (+ _startdrawpoint (* (`KismetMathLibrary.RotateAngleAxis` (`self.GetActorForwardVector` self) (`self.LCurrentAngle`) (0.0 0.0 1.0)) (`self.ExternalRadius`))) :`TraceChannel` "TraceTypeQuery1" :`DrawDebugType` (`self.Draw Debug Type`) :`DrawTime` (`self.Draw Time`)))
    (`KismetArrayLibrary.Array_Add` (`self.Out Hit`) _outhit))
  (`self.CreateProceduralMesh`))

(fn `InitializeFOV`
  (`|ExecutionSequence`
    (:`then_0`
      (bind _output_get (set `self.NumberOfSections` (`KismetMathLibrary.FCeil` (/ (* (`self.HalfAngle`) 2.0) (`self.DeltaAngle`)))))
      (set `self.DAngle` (/ (* (`self.HalfAngle`) 2.0) _output_get)))
    (:`then_1`
      (set `self.StartDrawPoint` (+ (`KismetMathLibrary.MakeVector` 0.0 0.0 (- (`self.HeightOfCheck`) 100.0)) (`self.K2_GetActorLocation` self))))
    (:`then_2`
      (`SceneComponent.K2_AddLocalOffset` (`self.ProceduralMesh`) (`KismetMathLibrary.MakeVector` 0.0 0.0 (- (`self.HeightOfShow`) 100.0)) false false))))

(fn `UpdateFOV`
  (set `self.StartDrawPoint` (+ (`KismetMathLibrary.MakeVector` 0.0 0.0 (- (`self.HeightOfCheck`) 100.0)) (`self.K2_GetActorLocation`)))
  (`KismetArrayLibrary.Array_Clear` (`self.Out Hit`))
  (`ProceduralMeshComponent.ClearAllMeshSections` (`self.ProceduralMesh`)))

(fn `UserConstructionScript`
  (if (`self.Rebuild`)
    (`self.InitializeFOV` self)
    (`self.Draw View Lines` self)))